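; End-of-level checkpoint that banks the character's cached score into the game instance's player info when the character overlaps its box.
; It rebuilds the saved high score list, adding the player's entry before any equal or higher score, or alone if no save exists.
; The list saves asynchronously and feeds an end-level widget shown with UI-only input.
; An EndLevel level load is left unconnected.
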(event OnComponentBeginOverlap(Box)
  (params (OverlappedComponent :type Primitive%20Component%20Object%20Reference) (OtherActor :type Actor%20Object%20Reference) (OtherComp :type Primitive%20Component%20Object%20Reference) (OtherBodyIndex :type Integer) (bFromSweep :type Boolean) (SweepResult :type Hit%20Result%20Structure%20%28by%20ref%29))
  (bind _returnvalue (Game|GetPlayerController 0))
  (bind _asthird_person_character (Utilities|Casting|CastToThirdPersonCharacter OtherActor))
  (bind _assetup_game_instance (Utilities|Casting|CastToSetup_GameInstance (Game|GetGameInstance)))
  (Variables|/Game/Levels/Setup_GameInstance.Setup_GameInstance_C|SetPlayerInfo _assetup_game_instance (Utilities|Struct|MakeStruct_PlayerInfo (.playername (Variables|/Game/Levels/Setup_GameInstance.Setup_GameInstance_C|GetPlayerInfo _assetup_game_instance)) (+ (.score (Variables|/Game/Levels/Setup_GameInstance.Setup_GameInstance_C|GetPlayerInfo _assetup_game_instance)) (Variables|/Game/ThirdPersonBP/Blueprints/ThirdPersonCharacter.ThirdPersonCharacter_C|GetCachedScore _asthird_person_character))))
  (Variables|/Game/ThirdPersonBP/Blueprints/ThirdPersonCharacter.ThirdPersonCharacter_C|SetCachedScore _asthird_person_character 0.0)
  (CallFunction|AddScoretoHighScoreList)
  (Viewport|RemoveAllWidgets)
  (bind _returnvalue_2 (UserInterface|CreateWidget "/Game/UI/WBP_EndLevel.WBP_EndLevel_C" 0 (Variables|Default|GetTemporary%20High%20Score%20List)))
  (UserInterface|Viewport|AddtoViewport _returnvalue_2 0)
  (Variables|/Script/Engine.PlayerController|SetbShowMouseCursor _returnvalue true)
  (Input|SetInputModeUIOnly _returnvalue _returnvalue_2 "DoNotLock"))

(event Custom|AddScoreToHighScoreList
  (bind _returnvalue (SaveGame|LoadGamefromSlot "HighScoreList_SaveGame"))
  (bind _ashigh_score_list_save_game (Utilities|Casting|CastToHighScoreList_SaveGame _returnvalue)
    (:then
      (for _array_element (Variables|/Game/Levels/HighScoreList_SaveGame.HighScoreList_SaveGame_C|GetHighScoreList _ashigh_score_list_save_game)
        (Development|PrintString (Utilities|String|Append "NAME: " (Utilities|String|ToString(Text) (.PlayerName (Utilities|Struct|BreakStruct_PlayerInfo _array_element))) ", SCORE: " (Utilities|String|ToString(Float) (.Score (Utilities|Struct|BreakStruct_PlayerInfo _array_element)))))
        (Utilities|FlowControl|Sequence
          (:then_0
            (bind _assetup_game_instance (Utilities|Casting|CastToSetup_GameInstance (Game|GetGameInstance)))
            (if (<= (.score (Variables|/Game/Levels/Setup_GameInstance.Setup_GameInstance_C|GetPlayerInfo _assetup_game_instance)) (.Score (Utilities|Struct|BreakStruct_PlayerInfo _array_element)))
              (Utilities|Array|Add (Variables|Default|GetTemporary%20High%20Score%20List) (Utilities|Struct|MakeStruct_PlayerInfo (.playername (Variables|/Game/Levels/Setup_GameInstance.Setup_GameInstance_C|GetPlayerInfo _assetup_game_instance)) (.score (Variables|/Game/Levels/Setup_GameInstance.Setup_GameInstance_C|GetPlayerInfo _assetup_game_instance))))
              (Utilities|FlowControl|DoOnce true)))
          (:then_1
            (Utilities|Array|Add (Variables|Default|GetTemporary%20High%20Score%20List) _array_element))))
      (bind _returnvalue_2 (SaveGame|CreateSaveGameObject "/Game/Levels/HighScoreList_SaveGame.HighScoreList_SaveGame_C" :!label _label))
      (Variables|/Game/Levels/HighScoreList_SaveGame.HighScoreList_SaveGame_C|SetHighScoreList _returnvalue_2 (Variables|Default|GetTemporary%20High%20Score%20List))
      (|AsyncSaveGametoSlot _returnvalue_2 "HighScoreList_SaveGame"))
    (:CastFailed
      (Utilities|FlowControl|Sequence
        (:then_0
          (Utilities|Array|Add (Variables|Default|GetTemporary%20High%20Score%20List) (Utilities|Struct|MakeStruct_PlayerInfo (.playername (Variables|/Game/Levels/Setup_GameInstance.Setup_GameInstance_C|GetPlayerInfo _assetup_game_instance)) (.score (Variables|/Game/Levels/Setup_GameInstance.Setup_GameInstance_C|GetPlayerInfo _assetup_game_instance))))
          (Utilities|FlowControl|DoOnce true))
        (:then_1
          (goto _label))))))

(fn ConstructionScript
  (|CallParentFunction))