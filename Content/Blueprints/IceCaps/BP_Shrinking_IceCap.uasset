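; BP_Shrinking_IceCap is an ice cap actor that shrinks while a player-distance check passes, then disappears.
; Tick calls CheckDistanceFromPlayer and, when true, runs MeltIceCap; BeginPlay and construction only call the parent versions.
; MeltIceCap subtracts a fixed amount from ObjectShape, applies it as the IceCap component's relative scale, and destroys the actor near zero.
; The melt step ignores delta time, so its speed depends on frame rate.
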(event Custom|MeltIceCap
  ;[1 1 1] Melt ice caps
  (bind _output_get (Variables|Default|SetObjectShape (+ (Variables|Default|GetObjectShape) "-0.001000,-0.001000,-0.001000")))
  (Transformation|SetRelativeScale3D (Variables|Default|GetIce%20Cap) _output_get)
  (if (Math|Vector|Equal(Vector) _output_get "0, 0,0.000000" 0.01)
    (Actor|DestroyActor)))

(event EventTick
  (params (DeltaSeconds :type Float%20%28single-precision%29))
  ;[1 1 1] Checks whether to begin melting ice cap
  (bind _hasactionbegun (CallFunction|CheckDistancefromPlayer))
  (if _hasactionbegun
    (CallFunction|MeltIceCap)))

(event EventBeginPlay
  ;[1 1 1] Get reference to player character + get size of object
  (|CallParentFunction))

(fn ConstructionScript
  (|CallParentFunction))