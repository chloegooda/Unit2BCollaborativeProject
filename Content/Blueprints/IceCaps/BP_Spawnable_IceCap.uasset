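; Spawnable ice cap actor with a player-proximity check for gating an action.
; BeginPlay caches the ThirdPersonCharacter through GetActorOfClass.
; CheckDistanceFromPlayer returns true when the player is closer than DistanceFromIceberg, or whenever HasActionBegun is already set.
; The action itself and the setting of that flag are not implemented in these graphs.
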(event EventBeginPlay
  ;[1 1 1] Get reference to player character + get size of object
  (bind _returnvalue (Actor|GetActorOfClass "/Game/ThirdPersonBP/Blueprints/ThirdPersonCharacter.ThirdPersonCharacter_C"))
  (Variables|Default|SetPlayerCharacter _returnvalue))

(fn ConstructionScript)

(fn CheckDistancefromPlayer
  (if (Variables|Default|GetHasActionBegun)
    (return true)
    (elif (and (< (Math|Vector|Distance(Vector) (Transformation|GetActorLocation self) (Transformation|GetActorLocation (Variables|Default|GetPlayerCharacter))) (Variables|Default|GetDistanceFromIceberg)) (not (Variables|Default|GetHasActionBegun)))
      (return true)
      (else
        (return false)))))