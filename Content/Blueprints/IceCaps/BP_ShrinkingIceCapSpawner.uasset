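; Spawner actor that creates BP_Shrinking_IceCap actors at its own location and rotation.
; On BeginPlay it caches its actor tags as CheckpointTags and prints each one.
; SpawnIceCap, which is not called within this Blueprint, spawns a cap scaled by IceCapSize with the spawner as owner.
; It then passes the cached tags to the new cap and applies IceCapMesh to its mesh component.
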(event EventBeginPlay
  (bind _output_get (Variables|Default|SetCheckpointTags (Variables|Actor|GetTags)))
  (for _array_element _output_get
    (Development|PrintString (Utilities|String|ToString(Name) _array_element))))

(event Collision|EventActorBeginOverlap
  (params (OtherActor :type Actor%20Object%20Reference)))

(event EventTick
  (params (DeltaSeconds :type Float%20%28single-precision%29)))

(fn ConstructionScript)

(fn SpawnIceCap
  (bind _returnvalue (Game|SpawnActorfromClass "/Game/Blueprints/IceCaps/BP_Shrinking_IceCap.BP_Shrinking_IceCap_C" (Math|Transform|MakeTransform (Transformation|GetActorLocation) (Transformation|GetActorRotation) (Variables|Default|GetIceCapSize)) "AdjustIfPossibleButAlwaysSpawn" self 0))
  (Variables|/Script/Engine.Actor|SetTags _returnvalue (Variables|Default|GetCheckpointTags))
  (Components|StaticMesh|SetStaticMesh (Variables|/Game/Blueprints/IceCaps/BP_Shrinking_IceCap.BP_Shrinking_IceCap_C|GetIce%20Cap _returnvalue) (Variables|Default|GetIce%20Cap%20Mesh)))