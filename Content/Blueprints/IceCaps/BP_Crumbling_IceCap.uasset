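; Crumbling ice cap Blueprint whose two breakable sections sink or shift vertically, then hide, once a player distance check triggers it.
; Tick calls the distance check and, when HasActionBegun is set, a DoOnce crumbles section 2, then section 1 after a delay, through one shared timeline.
; Reset applies the chosen iceberg mesh set, clears state and restores section visibility, collision and cached heights.
; The code that caches those heights is disconnected.
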(event Custom|BeginCrumble
  ;[1 1 1] Individually crumble sections
  (Utilities|FlowControl|DoOnce false
    (:Completed
      (CallFunction|CrumblingMovement (Variables|Default|GetCrumblingSection2))
      (Utilities|FlowControl|Delay 2.5)
      (CallFunction|CrumblingMovement (Variables|Default|GetCrumblingSection1)))))

(event Custom|Crumbling%20Movement
  (params (Crumbling%20Section :type Scene%20Component%20Object%20Reference))
  ;[1 1 1] Crumbling movement for sections
  (Variables|Default|SetIsCrumbled true)
  (if (Variables|Default|GetHasActionBegun)
    (bind _percentage (Timeline|Timeline_0 PlayFromStart)
      (:Update
        (if (Variables|Default|GetHasActionBegun)
          (Transformation|SetRelativeLocation Crumbling%20Section (Math|Vector|MakeVector 0.0 0.0 (* _percentage (Variables|Default|GetMovementHeight))) false false)
          (else
            (Timeline|Timeline_0 SetNewTime))))
      (:Finished
        (Rendering|SetVisibility Crumbling%20Section false true)))))

(event Custom|SetActiveCS
  (bind _crumblingsection1 (Variables|Default|GetCrumblingSection1))
  (bind _crumblingsection2 (Variables|Default|GetCrumblingSection2))
  ;[1 1 1] Resets ice berg
  (Collision|SetCollisionEnabled (Variables|Default|GetCrumblingSection1) "QueryAndPhysics")
  (Rendering|SetVisibility _crumblingsection1 true true)
  (Transformation|SetRelativeLocation _crumblingsection1 (Math|Vector|MakeVector 0.0 0.0 (Variables|Default|GetCachedHeightCS1)) false false)
  (Collision|SetCollisionEnabled (Variables|Default|GetCrumblingSection2) "QueryAndPhysics")
  (Rendering|SetVisibility _crumblingsection2 true true)
  (Transformation|SetRelativeLocation _crumblingsection2 (Math|Vector|MakeVector 0.0 0.0 (Variables|Default|GetCachedHeightCS2)) false false))

(event EventReset
  ;[1 1 1] Resets ice berg
  (CallFunction|SetUpMeshes (Variables|Default|GetTypeOfIceberg))
  (Variables|Default|SetIsCrumbled false)
  (Variables|Default|SetHasActionBegun false)
  (CallFunction|SetActiveCS)
  (Audio|Components|Audio|Stop (Variables|Default|GetTimeline_0))
  ;[1 1 1] Individually crumble sections
  (Utilities|FlowControl|DoOnce false) ; enters at Reset
)

(event EventTick
  (params (DeltaSeconds :type Float%20%28single-precision%29))
  ;[1 1 1] Checks whether to begin crumbling ice cap
  (CallFunction|CheckDistancefromPlayer)
  (if (Variables|Default|GetHasActionBegun)
    (CallFunction|BeginCrumble)))

(event EventBeginPlay
  ;[1 1 1] Get reference to player character+ reset
  (|CallParentFunction)
  (CallFunction|Reset))

(fn ConstructionScript
  (|CallParentFunction))

(fn SetUpMeshes
  (params (Type%20Of%20Iceberg :type Enum_CrumblingIcebergTypes%20Enum :default "NewEnumerator0"))
  (switch Utilities|FlowControl|Switch|SwitchonEnum_CrumblingIcebergTypes Type%20Of%20Iceberg
    (:NewEnumerator0
      (Components|StaticMesh|SetStaticMesh (Variables|Default|GetIce%20Cap) "/Game/Assets/Meshes/SM_Faller_01a.SM_Faller_01a")
      (Components|StaticMesh|SetStaticMesh (Variables|Default|GetCrumblingSection2) "/Game/Assets/Meshes/SM_Faller_01b.SM_Faller_01b")
      (Components|StaticMesh|SetStaticMesh (Variables|Default|GetCrumblingSection1) "/Game/Assets/Meshes/SM_Faller_01c.SM_Faller_01c"))
    (:NewEnumerator1
      (Components|StaticMesh|SetStaticMesh (Variables|Default|GetIce%20Cap) "/Game/Assets/Meshes/SM_Faller_02a.SM_Faller_02a")
      (Components|StaticMesh|SetStaticMesh (Variables|Default|GetCrumblingSection2) "/Game/Assets/Meshes/SM_Faller_02b.SM_Faller_02b")
      (Components|StaticMesh|SetStaticMesh (Variables|Default|GetCrumblingSection1) "/Game/Assets/Meshes/SM_Faller_02c.SM_Faller_02c")))
  (return))