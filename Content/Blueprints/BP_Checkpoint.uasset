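; BP_Checkpoint is a checkpoint that records a respawn point for the ThirdPersonCharacter and banks its score.
; On box overlap it stores itself and the location of its referenced CheckPointLocation actor on the character, then moves the character's cached score into the GameInstanceTest total.
; Its Reset event sends ResetMessage to every actor in ActorsToReset, restoring state tied to that checkpoint.
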(event OnComponentBeginOverlap(Box)
  (params (OverlappedComponent :type Primitive%20Component%20Object%20Reference) (OtherActor :type Actor%20Object%20Reference) (OtherComp :type Primitive%20Component%20Object%20Reference) (OtherBodyIndex :type Integer) (bFromSweep :type Boolean) (SweepResult :type Hit%20Result%20Structure%20%28by%20ref%29))
  (bind _asthird_person_character (Utilities|Casting|CastToThirdPersonCharacter OtherActor))
  (Variables|/Game/ThirdPersonBP/Blueprints/ThirdPersonCharacter.ThirdPersonCharacter_C|SetCheckPointLocation _asthird_person_character (Transformation|GetActorLocation (Variables|Default|GetCheckPointLocation)))
  (Variables|/Game/ThirdPersonBP/Blueprints/ThirdPersonCharacter.ThirdPersonCharacter_C|SetCheckPoint _asthird_person_character self)
  (bind _asgame_instance_test (Utilities|Casting|CastToGameInstanceTest (Game|GetGameInstance)))
  (Variables|/Game/Levels/GameInstanceTest.GameInstanceTest_C|SetScore _asgame_instance_test (+ (Variables|/Game/Levels/GameInstanceTest.GameInstanceTest_C|GetScore _asgame_instance_test) (Variables|/Game/ThirdPersonBP/Blueprints/ThirdPersonCharacter.ThirdPersonCharacter_C|GetCachedScore _asthird_person_character)))
  (Variables|/Game/ThirdPersonBP/Blueprints/ThirdPersonCharacter.ThirdPersonCharacter_C|SetCachedScore _asthird_person_character 0.0))

(event EventReset
  (for _array_element (Variables|Default|GetActorsToReset)
    (Class|BPICheckPoint|Reset(Message) _array_element)))

(fn ConstructionScript)