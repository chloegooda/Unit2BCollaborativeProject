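; A collectible item that adds a fixed amount to the ThirdPersonCharacter's cached score on overlap, then hides and disables its overlap box.
; Setup looks up its Type in DT_SpecialItems and, if found, stores the row, applies a hard-coded mesh and material, and re-enables the box.
; BeginPlay and Reset both run Setup, so collected items can reappear.
; StartFloating is empty, leaving the floating timeline unused.
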(event OnComponentBeginOverlap(Box)
  (params (OverlappedComponent :type Primitive%20Component%20Object%20Reference) (OtherActor :type Actor%20Object%20Reference) (OtherComp :type Primitive%20Component%20Object%20Reference) (OtherBodyIndex :type Integer) (bFromSweep :type Boolean) (SweepResult :type Hit%20Result%20Structure%20%28by%20ref%29))
  (bind _asthird_person_character (Utilities|Casting|CastToThirdPersonCharacter OtherActor))
  (Variables|/Game/ThirdPersonBP/Blueprints/ThirdPersonCharacter.ThirdPersonCharacter_C|SetCachedScore _asthird_person_character (+ (Variables|/Game/ThirdPersonBP/Blueprints/ThirdPersonCharacter.ThirdPersonCharacter_C|GetCachedScore _asthird_person_character) 88.0))
  (Rendering|SetVisibility (Variables|Default|GetBox) false true)
  (Variables|/Script/Engine.PrimitiveComponent|SetbGenerateOverlapEvents (Variables|Default|GetBox) false))

(event Custom|StartFloating
  ;[1 1 1] Start Floating
)

(event Custom|Setup
  (bind _cylinder (Variables|Default|GetCylinder))
  (CallFunction|StartFloating)
  (bind _returnvalue (Utilities|GetDataTableRow "/Game/Blueprints/Items/DT_SpecialItems.DT_SpecialItems" (Utilities|String|StringToName (Utilities|String|EnumtoString (Variables|Default|GetType))))
    (:then
      (Variables|Default|SetInfo _returnvalue)
      (Components|StaticMesh|SetStaticMesh _cylinder "/Game/Assets/Meshes/Old/SM_Peng_Spine.SM_Peng_Spine")
      (Rendering|Material|SetMaterial _cylinder 0 "/Game/Assets/Materials/Old/M_Orange.M_Orange")
      (Rendering|SetVisibility (Variables|Default|GetBox) true true)
      (Variables|/Script/Engine.PrimitiveComponent|SetbGenerateOverlapEvents (Variables|Default|GetBox) true))))

(event EventReset
  (CallFunction|Setup))

(event EventBeginPlay
  (CallFunction|Setup))

(fn ConstructionScript)