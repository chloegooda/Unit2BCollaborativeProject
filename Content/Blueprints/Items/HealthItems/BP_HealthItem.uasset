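; BP_HealthItem is a health pickup that restores player health when something overlaps its box.
; On BeginPlay it looks up its editor-set Type enum as a row name in DT_HealthItems, storing the row and applying its static mesh.
; On overlap it destroys itself, adds the row's restore amount to Health on GameInstanceTest and prints the new total, with no check on the overlapping actor.
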(event OnComponentBeginOverlap(Box)
  (params (OverlappedComponent :type Primitive%20Component%20Object%20Reference) (OtherActor :type Actor%20Object%20Reference) (OtherComp :type Primitive%20Component%20Object%20Reference) (OtherBodyIndex :type Integer) (bFromSweep :type Boolean) (SweepResult :type Hit%20Result%20Structure%20%28by%20ref%29))
  ;[1 1 1] Adds health to player's health on pickup
  (Actor|DestroyActor)
  (bind _asgame_instance_test (Utilities|Casting|CastToGameInstanceTest (Game|GetGameInstance)))
  (bind _output_get (Variables|/Game/Levels/GameInstanceTest.GameInstanceTest_C|SetHealth _asgame_instance_test (+ (Variables|/Game/Levels/GameInstanceTest.GameInstanceTest_C|GetHealth _asgame_instance_test) (.HealthRestored (Utilities|Struct|BreakStruct_HealthItems (Variables|Default|GetInfo))))))
  (Development|PrintString (Utilities|String|ToString(Float) _output_get)))

(event EventBeginPlay
  ;[1 1 1] Set up health item based off enum which is set in editor
  (bind _returnvalue (Utilities|GetDataTableRow "/Game/Blueprints/Items/HealthItems/DT_HealthItems.DT_HealthItems" (Utilities|String|StringToName (Utilities|String|EnumtoString (Variables|Default|GetType))))
    (:then
      (bind _output_get (Variables|Default|SetInfo _returnvalue))
      (Components|StaticMesh|SetStaticMesh (Variables|Default|GetItem) (.staticmesh _output_get)))))

(fn ConstructionScript)